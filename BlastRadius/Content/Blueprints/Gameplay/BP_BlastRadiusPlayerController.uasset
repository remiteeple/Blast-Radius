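; Player controller for Blast Radius that shows the match-start countdown and the team victory screens.
; BeginPlay shows 3, 2, 1 and Blast widgets for one second each using chained delays.
; Tick polls WinningTeam on the game state and creates an Orange or Blue wins widget, with no guard against re-creating it every frame.
; Health text and energy bar creation is present but never runs.
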(event EventBeginPlay
  (bind _returnvalue (UserInterface|CreateWidget "/Game/Blueprints/Menu/3HUD.3HUD_C"))
  (UserInterface|Viewport|AddtoPlayerScreen _returnvalue)
  (Utilities|FlowControl|Delay 1.0)
  (Widget|RemovefromParent _returnvalue)
  (bind _returnvalue_2 (UserInterface|CreateWidget "/Game/Blueprints/Menu/2HUD.2HUD_C"))
  (UserInterface|Viewport|AddtoPlayerScreen _returnvalue_2)
  (Utilities|FlowControl|Delay 1.0)
  (Widget|RemovefromParent _returnvalue_2)
  (bind _returnvalue_3 (UserInterface|CreateWidget "/Game/Blueprints/Menu/1HUD.1HUD_C"))
  (UserInterface|Viewport|AddtoPlayerScreen _returnvalue_3)
  (Utilities|FlowControl|Delay 1.0)
  (Widget|RemovefromParent _returnvalue_3)
  (bind _returnvalue_4 (UserInterface|CreateWidget "/Game/Blueprints/Menu/BlastHUD.BlastHUD_C"))
  (UserInterface|Viewport|AddtoPlayerScreen _returnvalue_4)
  (Utilities|FlowControl|Delay 1.0)
  (Widget|RemovefromParent _returnvalue_4))

(event EventTick
  (params (DeltaSeconds :type Float%20%28single-precision%29))
  (bind _asblast_radius_game_state_base (Utilities|Casting|CastToBlastRadiusGameStateBase (Game|GetGameState)))
  (Math|Integer|CompareInt (Variables|/Script/BlastRadius.BlastRadiusGameStateBase|GetWinningTeam _asblast_radius_game_state_base)
    (:>
      (bind _returnvalue (UserInterface|CreateWidget "/Game/Blueprints/Menu/OrangeWinsHUD.OrangeWinsHUD_C"))
      (UserInterface|Viewport|AddtoPlayerScreen _returnvalue))
    (:==
      (bind _returnvalue_2 (UserInterface|CreateWidget "/Game/Blueprints/Menu/BlueWinsHUD.BlueWinsHUD_C"))
      (UserInterface|Viewport|AddtoPlayerScreen _returnvalue_2))))

(fn ConstructionScript)